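; BP_Soldier is a Paper2D soldier character that handles weapon-based sprite visuals and a death effect on top of a parent soldier class.
; Every tick it picks the pistol or SMG flipbook from the active gun's type.
; On death it stops ticking, lowers itself, swaps to a shrunken, red-tinted splatter flipbook, then calls the parent death logic after a short delay.
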(event `self.ReceiveBeginPlay`)

(event `self.ReceiveTick`
  (params (DeltaSeconds :type "Float (single-precision)"))
  (bind _paperflipbook (`self.PaperFlipbook`))
  (bind _returnvalue (`Gun.GetType` (`self.ActiveGun`)))
  (switch `EGunType` _returnvalue
    (:`Pistol`
      (`TankStatics.PlayFlipbook` _paperflipbook "/Game/Textures/Characters/Character_0_Pistol.Character_0_Pistol"))
    (:`SMG`
      (`TankStatics.PlayFlipbook` _paperflipbook "/Game/Textures/Characters/Character_0_SMG.Character_0_SMG"))))

(event `self.SoldierDie`
  (params (DamageType :type "EDamageType Enum" :default "Uknown"))
  (bind _paperflipbook (`self.PaperFlipbook`))
  (`self.K2_AddActorLocalOffset` (0.0 0.0 -10.0))
  (`self.SetActorTickEnabled` false)
  (`TankStatics.PlayFlipbook` _paperflipbook "/Game/Textures/Splats/Spla00_Flipbook.Spla00_Flipbook")
  (`PaperFlipbookComponent.SetSpriteColor` _paperflipbook (struct :`R` 0.570833 :`G` 0.014523 :`B` 0.009514 :`A` 1.0))
  (`SceneComponent.SetRelativeScale3D` _paperflipbook (0.5 0.5 0.5))
  (`KismetSystemLibrary.Delay` 3.0)
  (`parent.SoldierDie` DamageType))

(fn `UserConstructionScript`)