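; Tank Blueprint built on Paper2D components that adds a visual death sequence to its parent class's TankDie event.
; On death it plays an explosion flipbook, hides the child turret and fades the tank sprite's alpha through a timeline.
; The parent TankDie is deferred until the explosion's finished-playing callback fires, so inherited death handling runs after the animation.
; BeginPlay, Tick, overlap and construction script are empty.
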(event `self.ReceiveBeginPlay`)

(event `self.TankDie`
  (params (DamageType :type "EDamageType Enum" :default "Unknown"))
  (bind _explosion (`self.Explosion`))
  (`TankStatics.PlayFlipbook` _explosion "/Game/Sprites/Explosions/Explosion_2/Explosion.Explosion")
  (add `PaperFlipbookComponent.OnFinishedPlaying` _explosion (delegate `On Finished Playing`))
  (`SceneComponent.SetHiddenInGame` (`self.ChildTurret`) true false)
  (bind (_direction _fade_value) (`Timeline|Fade timelien`)
    (:`Update`
      (`PaperSpriteComponent.SetSpriteColor` (`self.TankSprite`) (`KismetMathLibrary.MakeColor` 1.0 1.0 1.0 _fade_value)))))

(event `On Finished Playing`
  (`parent.TankDie` (stale `self.TankDie` DamageType)))

(fn `UserConstructionScript`)