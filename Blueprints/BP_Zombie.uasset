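; Paper2D zombie Blueprint that supplies the flipbook visuals for the walk, attack, run and death events.
; Walk playback rate scales with movement speed between the walk and run speeds.
; On death it disables collision and tick, lowers the actor and shows a rescaled splat flipbook.
; A timeline animates the alpha of the green-tinted splat, then calls the parent death handler when finished.
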(event `self.ReceiveBeginPlay`)

(event `self.ReceiveTick`
  (params (DeltaSeconds :type "Float (single-precision)")))

(event `self.ZombieWalk`
  (params (DeltaTime :type "Float (single-precision)") (DistanceWalkedThisFrame :type "Vector Structure"))
  (`TankStatics.PlayFlipbook` (`self.PaperFlipbook`) "/Game/Textures/Characters/Zombie_Walk.Zombie_Walk" true (`KismetMathLibrary.MapRangeClamped` (/ (`KismetMathLibrary.VSize` DistanceWalkedThisFrame) DeltaTime) (`self.WalkSpeed`) (`self.RunSpeed`) 1.0 2.0)))

(event `self.ZombieAttack`
  (params (DeltaTime :type "Float (single-precision)"))
  (`TankStatics.PlayFlipbook` (`self.PaperFlipbook`) "/Game/Textures/Characters/Zombie_Attack.Zombie_Attack" true))

(event `self.ZombieRun`
  (params (DeltaTime :type "Float (single-precision)"))
  (`TankStatics.PlayFlipbook` (`self.PaperFlipbook`) "/Game/Textures/Characters/Zombie_Chase.Zombie_Chase" true))

(event `self.ZombieDie`
  (params (DamageType :type "EDamageType Enum" :default "Unknown"))
  (bind _paperflipbook (`self.PaperFlipbook`))
  (`self.SetActorEnableCollision` false)
  (`self.K2_AddActorWorldOffset` (0.0 0.0 -10.0))
  (`TankStatics.PlayFlipbook` _paperflipbook "/Game/Textures/Splats/Spla00_Flipbook.Spla00_Flipbook" true)
  (`self.SetActorTickEnabled` false)
  (`SceneComponent.SetRelativeScale3D` _paperflipbook (0.5 0.5 0.5))
  (`|ExecutionSequence`
    (:`then_0`
      (bind (_direction _newtrack_3) (`Timeline|Timeline_0`)
        (:`Update`
          (`PaperFlipbookComponent.SetSpriteColor` (`self.PaperFlipbook`) (* (`KismetMathLibrary.MakeColor` 1.0 1.0 1.0 _newtrack_3) (struct :`R` 0.024158 :`G` 0.417885 :`B` 0.116971 :`A` 1.0))))
        (:`Finished`
          (`parent.ZombieDie` DamageType))))))

(fn `UserConstructionScript`)