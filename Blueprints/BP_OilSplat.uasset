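; Flammable oil splat that a missile ignites on overlap, destroying the missile.
; Ignition swaps the oil sprite for a fire flipbook, enables a child DamageVolume and starts an alpha fade that ends in self-destruction; unlit splats fade after a timer.
; While burning with collision on, Tick box-traces to ignite overlapping splats, disabling their collision and then its own, so they do not trace further.
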(event `FadeOut`
  (bind _fireflipbook (`self.FireFlipbook`))
  (bind _oilsplatsprite (`self.OilSplatSprite`))
  (bind (_r _g _b) (`KismetMathLibrary.BreakColor` (`PaperFlipbookComponent.SpriteColor` _fireflipbook)))
  (bind (_r_2 _g_2 _b_2) (`KismetMathLibrary.BreakColor` (`PaperSpriteComponent.SpriteColor` _oilsplatsprite)))
  (bind (_direction _newtrack_0) (`Timeline|Timeline_1` :!via `PlayFromStart`)
    (:`Update`
      (`|ExecutionSequence`
        (:`then_0`
          (`PaperFlipbookComponent.SetSpriteColor` _fireflipbook (`KismetMathLibrary.MakeColor` _r _g _b _newtrack_0)))
        (:`then_1`
          (`PaperSpriteComponent.SetSpriteColor` _oilsplatsprite (`KismetMathLibrary.MakeColor` _r_2 _g_2 _b_2 _newtrack_0)))))
    (:`Finished`
      (`self.K2_DestroyActor`))))

(event `self.ReceiveBeginPlay`
  (add `self.StartFireDispatcher` (delegate `StartFire`))
  (add `self.FadeOutDispatcher` (delegate `FadeOut`))
  (`KismetSystemLibrary.K2_SetTimerDelegate` (delegate `FadeOut`) 30.0))

(event `StartFire`
  (`SceneComponent.SetVisibility` (`self.FireFlipbook`) true false)
  (`SceneComponent.SetVisibility` (`self.OilSplatSprite`) false false)
  (bind _asdamage_volume (cast `DamageVolume` (`ChildActorComponent.ChildActor` (`self.DamageVolume`))))
  (set `DamageVolume.bEnabled` true _asdamage_volume)
  (`self.FadeOutDispatcher`))

(event `self.FireTrigger.OnComponentBeginOverlap`
  (params (OverlappedComponent :type "PrimitiveComponent Object Reference") (OtherActor :type "Actor Object Reference") (OtherComp :type "PrimitiveComponent Object Reference") (OtherBodyIndex :type Integer) (bFromSweep :type Boolean) (SweepResult :type "HitResult Structure (by ref)"))
  (bind _asmissile (cast `Missile` OtherActor))
  (`Projectile.DestroyProjectile` _asmissile)
  (`self.StartFireDispatcher`))

(event `self.ReceiveTick`
  (params (DeltaSeconds :type "Float (single-precision)"))
  (bind _returnvalue (`self.K2_GetActorLocation`))
  (if (and (`self.GetActorEnableCollision`) (`SceneComponent.bVisible` (`self.FireFlipbook`)))
    (bind _outhits (`KismetSystemLibrary.BoxTraceMultiForObjects` _returnvalue _returnvalue (`BoxComponent.BoxExtent` (`self.FireTrigger`)) (struct) (`self.Object Query Array`)))
    (for _array_element _outhits
      (bind (_bblockinghit _binitialoverlap _time _distance _location _impactpoint _normal _impactnormal _physmat _hitactor) (`GameplayStatics.BreakHitResult` _array_element))
      (bind _asbp_oil_splat (cast `/Blueprints/BP_OilSplat` _hitactor))
      (`self.StartFireDispatcher` _asbp_oil_splat)
      (`self.SetActorEnableCollision` _hitactor false))
    (`self.SetActorEnableCollision` false)))

(fn `UserConstructionScript`)